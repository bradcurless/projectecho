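; BP_RoomGenerator is a level chunk Blueprint for a room with up to four openable door walls, configured at construction time.
; The construction script teleports each door wall flagged open to its offset as a relative location, leaving the others untouched.
; DoorDirection supplies that location, inverting the offset when the shared NegateDoorDir flag is set.
; The event graph has no active logic, so doors do not move during play.
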(event EventBeginPlay)

(event Collision|EventActorBeginOverlap
  (params (OtherActor :type Actor%20Object%20Reference)))

(event EventTick
  (params (DeltaSeconds :type Float%20%28single-precision%29)))

(fn ConstructionScript
  (if (Variables|Default|GetOpenDoor1)
    (bind _outdir (CallFunction|DoorDirection (Variables|Default|GetDoor1%20Offset)))
    (Transformation|SetRelativeLocation (Variables|Default|GetDoor%20Wall%201) _outdir false true))
  (if (Variables|Default|GetOpenDoor2)
    (bind _outdir_2 (CallFunction|DoorDirection (Variables|Default|GetDoor2%20Offset)))
    (Transformation|SetRelativeLocation (Variables|Default|GetDoor%20Wall%202) _outdir_2 false true))
  (if (Variables|Default|GetOpenDoor3)
    (bind _outdir_3 (CallFunction|DoorDirection (Variables|Default|GetDoor3%20Offset)))
    (Transformation|SetRelativeLocation (Variables|Default|GetDoor%20Wall%203) _outdir_3 false true))
  (if (Variables|Default|GetOpenDoor4)
    (bind _outdir_4 (CallFunction|DoorDirection (Variables|Default|GetDoor4%20Offset)))
    (Transformation|SetRelativeLocation (Variables|Default|GetDoor%20Wall%204) _outdir_4 false true)))

(fn DoorDirection
  (params (Direction :type Vector))
  (bind _output_get (LocalVariables|SetFinalDirection Direction))
  (if (Variables|Default|GetNegateDoorDir)
    (LocalVariables|SetFinalDirection (* _output_get -1.0)))
  (return (LocalVariables|GetFinalDirection)))